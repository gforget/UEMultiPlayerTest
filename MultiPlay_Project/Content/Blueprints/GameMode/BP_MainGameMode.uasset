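; Multiplayer game mode that tracks connected BP_MainPlayerController instances and supports kicking players.
; PostLogin and OnLogout add or remove controllers in the JoinedPlayer array, then call UpdatePlayerLIst.
; That event waits briefly before telling BP_MainGameState to refresh its player list.
; KickPlayer treats the given ID as an index into JoinedPlayer and calls OwningClientKickPlayer on that controller.
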(event `self.K2_PostLogin`
  (params (NewPlayer :type "PlayerController Object Reference"))
  (bind _asbp_main_player_controller (cast `/Game/Blueprints/Controller/BP_MainPlayerController` NewPlayer))
  (`KismetArrayLibrary.Array_Add` (`self.JoinedPlayer`) _asbp_main_player_controller)
  (`self.UpdatePlayerLIst`))

(event `self.K2_OnLogout`
  (params (ExitingController :type "Controller Object Reference"))
  (cast `/Game/Blueprints/Controller/BP_MainPlayerController` ExitingController)
  (`KismetArrayLibrary.Array_RemoveItem` (`self.JoinedPlayer`))
  (`self.UpdatePlayerLIst`))

(event `UpdatePlayerLIst`
  (`KismetSystemLibrary.Delay` 0.5)
  (bind _asbp_main_game_state (cast `/Game/Blueprints/GameMode/BP_MainGameState` (`GameplayStatics.GetGameState`)))
  (`/Game/Blueprints/GameMode/BP_MainGameState.UpdatePlayerList` _asbp_main_game_state))

(fn `KickPlayer`
  (params (PlayerId :type Integer))
  (`/Game/Blueprints/Controller/BP_MainPlayerController.OwningClient_KickPlayer` (`|GetArrayItem` (`self.JoinedPlayer`) PlayerId)))

(fn `UserConstructionScript`)